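; Animation notify that fires a peacock-pattern bullet-hell projectile volley from an animated mesh.
; On trigger, it finds the AC_BulletHell_Pro component on the mesh's owner and, if valid, calls SpawnPeacockProjectile.
; The notify's variables set the pattern's count, rate, speed, spread and angles, while a named socket supplies the start location.
; The first player's pawn is passed as the homing target.
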(fn `Received_Notify`
  (params (MeshComp :type "SkeletalMeshComponent Object Reference") (Animation :type "AnimSequenceBase Object Reference"))
  (returns (ReturnValue :type Boolean))
  (bind _returnvalue (`Actor.GetComponentByClass` (`ActorComponent.GetOwner` MeshComp) "/Game/BulletHell_Pro/Component/AC_BulletHell_Pro.AC_BulletHell_Pro_C"))
  (`/Engine/EditorBlueprintResources/StandardMacros.IsValid` _returnvalue
    (:`Is Valid`
      (`/Game/BulletHell_Pro/Component/AC_BulletHell_Pro.Spawn Peacock Projectile` _returnvalue (`self.Spawn Count`) (`self.Spawn Rate`) (`SceneComponent.GetSocketLocation` MeshComp (`self.In Socket Name`)) (`self.Projectile`) (`self.Projectile Speed`) (`self.Projectile H Sections`) (`self.Projectile Spread`) (`self.AngleDirection`) (`self.Pojectile Pitch`) (`self.Pojectile Yaw`) (`self.Start Z Offset`) (`GameplayStatics.GetPlayerPawn` 0))
      (return false))
    (:`Is Not Valid`
      (return false))))