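; Example turret that fires a bullet-hell pattern through its ACBulletHellPro component.
; FireProjectilesEvent, which nothing in this graph calls, waits a tiny random delay, then confirms the player pawn is BP_ThirdPersonCharacter.
; It then spawns a peacock spread of BP_Projectile_05 from the Arrow's location, with the player as homing target.
; Unwired arc, shockwave, direct, grid and peacock spawner nodes show the component's other options.
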(event `Fire Projectiles Event`
  (bind _returnvalue (`GameplayStatics.GetPlayerPawn` 0))
  ;[1 1 1] Turret fire event example
  (`KismetSystemLibrary.Delay` (`KismetMathLibrary.RandomFloatInRange` 0.0 0.02))
  (cast `/Game/BulletHell_Pro/Demo_Assets/ThirdPersonBP/Blueprints/BP_ThirdPersonCharacter` _returnvalue)
  (`/Game/BulletHell_Pro/Component/AC_BulletHell_Pro.Spawn Peacock Projectile` (`self.AC_BulletHell_Pro`) 2 0.4 (`SceneComponent.K2_GetComponentLocation` (`self.Arrow`)) "/Game/BulletHell_Pro/Component/Projectiles/BossProjectiles/BP_Projectile_05.BP_Projectile_05_C" 1400.0 9 1000.0 360.0 90.0 0.0 100.0 _returnvalue))

(fn `UserConstructionScript`)